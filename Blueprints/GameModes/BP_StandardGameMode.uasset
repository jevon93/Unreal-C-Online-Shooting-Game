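; BP_StandardGameMode is a game mode that randomly assigns each player a role, name and index.
; PostLogin adds each new controller to a Players array and reshuffles it, so array position supplies the randomness.
; Five seconds after BeginPlay, it copies the matching Roles and PlayerNamesList entries onto each BP_PlayerController.
; It also writes the array index to each controller and its BP_SpaceMarine pawn for character material selection.
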(event `self.ReceiveBeginPlay`
  ;[1 1 1] Set Player Role
  (`KismetSystemLibrary.Delay` 5.0)
  (for (_array_element _array_index) (`self.Players`)
    (bind _asbp_player_controller (cast `/Game/Blueprints/PlayerController/BP_PlayerController` _array_element))
    (set `/Game/Blueprints/PlayerController/BP_PlayerController.PC_Role` (`|GetArrayItem` (`self.Roles`) _array_index) _asbp_player_controller))
  ;[1 1 1] Set Random Player Name
  (for (_array_element_2 _array_index_2) (`self.Players`)
    (bind _asbp_player_controller_2 (cast `/Game/Blueprints/PlayerController/BP_PlayerController` _array_element_2))
    (set `/Game/Blueprints/PlayerController/BP_PlayerController.PC_PlayerName` (`|GetArrayItem` (`self.PlayerNamesList`) _array_index_2) _asbp_player_controller_2))
  ;[1 1 1] Set Player Index Number, Used for Selecting Player Character Material
  (for (_array_element_3 _array_index_3) (`self.Players`)
    (bind _asbp_player_controller_3 (cast `/Game/Blueprints/PlayerController/BP_PlayerController` _array_element_3))
    (set `/Game/Blueprints/PlayerController/BP_PlayerController.Index` _array_index_3 _asbp_player_controller_3)
    (bind _asbp_space_marine (cast `/Game/Blueprints/Character/BP_SpaceMarine` (`Controller.K2_GetPawn` _asbp_player_controller_3)))
    (set `/Game/Blueprints/Character/BP_SpaceMarine.Index` _array_index_3 _asbp_space_marine)))

(event `self.K2_PostLogin`
  (params (NewPlayer :type "PlayerController Object Reference"))
  ;[1 1 1] Create Array of Player Controllers on Login, Shuffle Index
  (`KismetArrayLibrary.Array_Add` (`self.Players`) NewPlayer)
  (`KismetArrayLibrary.Array_Shuffle` (`self.Players`)))

(fn `UserConstructionScript`)