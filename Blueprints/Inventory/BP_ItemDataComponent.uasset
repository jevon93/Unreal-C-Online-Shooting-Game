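; Item data component that turns its owning actor into a pickup for the player's inventory.
; On BeginPlay it makes the owner replicate.
; Interacting passes its item row name and quantity to the player character's inventory system and destroys the owner if the add succeeds.
; Its LookAt function returns an empty string.
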(event `self.ReceiveBeginPlay`
  (`Actor.SetReplicates` (`self.GetOwner`) true))

(event `/Game/Blueprints/Inventory/BP_InteractInterface.InteractWith`
  (params (PlayerCharacter :type "/Game/Blueprints/Character/BP_SpaceMarine Object Reference"))
  (bind _bp_inventorysystem (`/Game/Blueprints/Character/BP_SpaceMarine.BP_InventorySystem` PlayerCharacter))
  (bind (_itemid_datatable _itemid_rowname) (break `DataTableRowHandle` (`self.ItemID`)))
  (`/Engine/EditorBlueprintResources/StandardMacros.IsValid` _bp_inventorysystem
    (:`Is Valid`
      (bind _success (`/Game/Blueprints/Inventory/BP_InventorySystem.AddToInventory` _bp_inventorysystem _itemid_rowname (`self.Quantity`)))
      (if _success
        (`Actor.K2_DestroyActor` (`self.GetOwner`))))))

(fn `LookAt`
  (returns (Message :type Text))
  (return ""))