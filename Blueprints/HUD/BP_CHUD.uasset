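; BP_CHUD is a HUD Blueprint that creates and displays the hotbar, player menu and container inventory widgets.
; Separate events create each widget and add it to the viewport, storing the hotbar in its own variable.
; The player menu and container screen share one Menu variable, and ShowContainer passes the supplied inventory component into its widget.
; Neither menu event removes the previous widget before replacing that reference.
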(event `CustomEvent`
  (bind _returnvalue (`|CreateWidget` "/Game/Blueprints/Inventory/UI/Hotbar/WBP_Hotbar.WBP_Hotbar_C"))
  (bind _output_get (set `self.Hotbar Widget` _returnvalue))
  (`UserWidget.AddToViewport` _output_get 0))

(event `DisplayPlayerMenu`
  (bind _returnvalue (`|GenericCreateObject` "/Game/Blueprints/Inventory/UI/WBP_PlayerMenu.WBP_PlayerMenu_C"))
  (bind _output_get (set `self.Menu` _returnvalue))
  (`UserWidget.AddToViewport` _output_get 0))

(event `ShowContainer`
  (params (ContainerInventorySystem :type "/Game/Blueprints/Inventory/BP_InventorySystem Object Reference"))
  (bind _returnvalue (`|CreateWidget` "/Game/Blueprints/Inventory/UI/WBP_ContainerInventory.WBP_ContainerInventory_C" null ContainerInventorySystem))
  (bind _output_get (set `self.Menu` _returnvalue))
  (`UserWidget.AddToViewport` _output_get 0))

(fn `UserConstructionScript`)