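; Player controller that handles multiplayer text chat, the player HUD and inventory shortcuts.
; On BeginPlay, after a delay, the local controller creates the chat panel and HUD, while Enter opens a focused chat input box.
; SR_SubmitChat relays messages server-side by looping over the PlayerArray and calling each controller's client update on its chat panel.
; Inputs open the HUD's player menu or consume a hotbar item through the Space Marine's inventory system.
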(event `SR_SubmitChat`
  (params (PlayerName :type Text) (ChatMessage :type Text) (SendingPlayerIndex :type "SlateColor Structure") (PlayerRole :type Text))
  ;[1 1 1] Run Server Chat Update and Client Chat Update
  (for (_ _array_index) (`GameStateBase.PlayerArray` (`GameplayStatics.GetGameState`))
    (bind _asbp_player_controller (cast `/Blueprints/PlayerController/BP_PlayerController` (`GameplayStatics.GetPlayerController` _array_index)))
    (`self.OC_UpdateChat` _asbp_player_controller PlayerName ChatMessage SendingPlayerIndex PlayerRole)))

(event `OC_UpdateChat`
  (params (PlayerName :type Text) (ChatMessage :type Text) (SendingPlayerIndex :type "SlateColor Structure") (PlayerRole :type Text))
  ;[1 1 1] Run Server Chat Update and Client Chat Update
  (bind _wb_chatpanel (`self.WB_ChatPanel`)
    (:`then`
      (`/Game/Blueprints/MultiplayerChat/WB_ChatPanel.Update_Chat` _wb_chatpanel PlayerName ChatMessage SendingPlayerIndex PlayerRole))
    (:`else`)))

(event `Key|Enter`
  (params (Key :type "Key Structure"))
  ;[1 1 1] Create Chat Message Input on Enter Key Pressed
  (:`Pressed`
    (if (`self.IsLocalPlayerController`)
      (bind _returnvalue (`|CreateWidget` "/Game/Blueprints/MultiplayerChat/WB_ChatInputBox.WB_ChatInputBox_C" self))
      (bind _output_get (set `self.WB_ChatInput` _returnvalue))
      (`UserWidget.AddToViewport` _output_get 0)
      (`Widget.SetKeyboardFocus` (`/Game/Blueprints/MultiplayerChat/WB_ChatInputBox.ChatInputBox` _output_get)))))

(event `self.ReceiveBeginPlay`
  ;[1 1 1] Create Chat Panel Widget
  (`KismetSystemLibrary.Delay` 7.0)
  (if (`self.IsLocalPlayerController`)
    (bind _returnvalue (`|CreateWidget` "/Game/Blueprints/MultiplayerChat/WB_ChatPanel.WB_ChatPanel_C" self))
    (bind _output_get (set `self.WB_ChatPanel` _returnvalue))
    (`UserWidget.AddToViewport` _output_get 0)
    (if (`self.IsLocalPlayerController`)
      (bind _returnvalue_2 (`|CreateWidget` "/Game/Blueprints/HUD/WBP_PlayerHUD.WBP_PlayerHUD_C" null null null))
      (bind _output_get_2 (set `self.WB_HUD` _returnvalue_2))
      (`UserWidget.AddToViewport` _output_get_2 0))))

(event `InputAction|Inventory`
  (params (Key :type "Key Structure"))
  (:`Pressed`
    (`/Game/Blueprints/HUD/WBP_PlayerHUD.DisplayPlayerMenu` (`self.WB_HUD`))))

(event `InputAction|Hotbar4`
  (params (Key :type "Key Structure"))
  (:`Pressed`
    (bind _asbp_space_marine (cast `/Game/Blueprints/Character/BP_SpaceMarine` (`self.K2_GetPawn`)))
    (`/Game/Blueprints/Inventory/BP_InventorySystem.ConsumeItem` (`/Game/Blueprints/Character/BP_SpaceMarine.BP_InventorySystem` _asbp_space_marine) (`/Game/Blueprints/Inventory/UI/Hotbar/WBP_HotBarSlot.InventoryIndex` (`/Game/Blueprints/Inventory/UI/Hotbar/WBP_Hotbar.WBP_HotBarSlot_3` (`/Game/Blueprints/HUD/WBP_PlayerHUD.Hotbar Widget` (`self.WB_HUD`)))))))

(fn `UserConstructionScript`)