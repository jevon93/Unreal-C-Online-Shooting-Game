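; BP_SpaceMarine is a space marine character Blueprint that colours its mesh per player.
; On BeginPlay it waits a fixed delay, then sets the mesh's first material slot to the PlayerColours entry selected by Index.
; Index has a RepNotify function, but it is empty, so the colour is applied only by that delayed step.
; Logic to show the net role on an overhead widget is present but disconnected.
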(event `self.ReceiveBeginPlay`
  (`KismetSystemLibrary.Delay` 7.0)
  (`PrimitiveComponent.SetMaterial` (`self.Mesh`) 0 (`|GetArrayItem` (`self.PlayerColours`) (`self.Index`))))

(fn `OnRep_Index`)

(fn `UserConstructionScript`)